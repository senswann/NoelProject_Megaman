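; Base enemy actor that takes damage from projectiles and hurts the hero on contact.
; Overlaps with BP_NBG_Projectiles on its collision component subtract projectile damage from HP, while capsule hits on BP_HeroCharacter deal its own damage.
; When a hit would deplete HP, Death rolls random loot (a medium or default health boost, a point coin, or nothing) and destroys the actor.
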(event OnComponentBeginOverlap(Colision)
  (params (OverlappedComponent :type Primitive%20Component%20Object%20Reference) (OtherActor :type Actor%20Object%20Reference) (OtherComp :type Primitive%20Component%20Object%20Reference) (OtherBodyIndex :type Integer) (bFromSweep :type Boolean) (SweepResult :type Hit%20Result%20Structure%20%28by%20ref%29))
  ;[1 1 1] If hit
  (bind _asbp_nbg_projectiles (Utilities|Casting|CastToBP_NBG_Projectiles OtherActor))
  (CallFunction|GetDamage (Variables|/Script/NoeldesBG.NBG_Projectiles|GetDammage _asbp_nbg_projectiles)))

(event OnComponentHit(CapsuleComponent)
  (params (HitComponent :type Primitive%20Component%20Object%20Reference) (OtherActor :type Actor%20Object%20Reference) (OtherComp :type Primitive%20Component%20Object%20Reference) (NormalImpulse :type Vector :default "0, 0, 0") (Hit :type Hit%20Result%20Structure%20%28by%20ref%29))
  ;[1 1 1] if touch player
  (bind _asbp_hero_character (Utilities|Casting|CastToBP_HeroCharacter OtherActor))
  (Default|GetDammage _asbp_hero_character (Variables|Default|GetDammage)))

(event EventBeginPlay)

(event Collision|EventActorBeginOverlap
  (params (OtherActor :type Actor%20Object%20Reference)))

(event EventTick
  (params (DeltaSeconds :type Float%20%28single-precision%29)))

(fn ConstructionScript)

(fn GetDamage
  (params (Degat :type Integer))
  (if (> (- (Variables|Default|GetHP) Degat) 0)
    (Variables|Default|SetHP (- (Variables|Default|GetHP) Degat))
    (else
      (CallFunction|Death))))

(fn Death
  (bind _returnvalue (Transformation|GetActorTransform))
  (switch int (Math|Random|RandomIntegerinRange 0 10)
    (:Default
      _)
    (:0
      (bind _returnvalue_2 (Game|SpawnActorfromClass "/Game/ProjetNoel/Blueprint/Items/Bonus/BP_NBG_HealthBoost.BP_NBG_HealthBoost_C" _returnvalue "Undefined" "MultiplyWithRoot" 0 0))
      (Variables|/Script/NoeldesBG.HealthBoost|SetIsHPMedium _returnvalue_2 true))
    (:1
      (Game|SpawnActorfromClass "/Game/ProjetNoel/Blueprint/Items/Bonus/BP_NBG_HealthBoost.BP_NBG_HealthBoost_C" _returnvalue "Undefined" "MultiplyWithRoot" 0 0))
    (:2
      (Game|SpawnActorfromClass "/Game/ProjetNoel/Blueprint/Items/Bonus/BP_NBG_PointCoins.BP_NBG_PointCoins_C" _returnvalue "Undefined" "MultiplyWithRoot" 0 0 :!label _label))
    (:3
      (goto _label))
    (:4
      (goto _label))
    (:5
      (goto _label)))
  (Actor|DestroyActor))