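; BP_AiBase_Flying is a flying enemy base that runs the BT_FlyingAi behavior tree on BeginPlay.
; PawnSensing sets the IsSeePlayer blackboard key when it sees a pawn, and a collision overlap with the hero character clears it.
; The construction script reads HP and damage from DT_NBG_Value, stores the starting transform, and builds a two-point relative InterpToMovement path from Locations.
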(event OnSeePawn(PawnSensing)
  (params (Pawn :type Pawn%20Object%20Reference))
  ;[1 1 1] ifSeePlayer
  (AI|Components|Blackboard|SetValueasBool (AI|GetBlackboard (AI|GetAIController self)) (Utilities|Name|MakeLiteralName "IsSeePlayer") true))

(event OnComponentBeginOverlap(Colision)
  (params (OverlappedComponent :type Primitive%20Component%20Object%20Reference) (OtherActor :type Actor%20Object%20Reference) (OtherComp :type Primitive%20Component%20Object%20Reference) (OtherBodyIndex :type Integer) (bFromSweep :type Boolean) (SweepResult :type Hit%20Result%20Structure%20%28by%20ref%29))
  (Utilities|Casting|CastToBP_NBG_HeroCharacter OtherActor)
  (AI|Components|Blackboard|SetValueasBool (AI|GetBlackboard (AI|GetAIController self)) (Utilities|Name|MakeLiteralName "IsSeePlayer") false))

(event EventBeginPlay
  (|CallParentFunction)
  (AI|RunBehaviorTree (AI|GetAIController self) "/Game/ProjetNoel/Blueprint/Ennemi/BehaviorTree/FlyAi/BT_FlyingAi.BT_FlyingAi"))

(fn ConstructionScript
  (bind _locations (Variables|Default|GetLocations))
  (bind _interptomovement (Variables|Default|GetInterpToMovement))
  (|CallParentFunction)
  (bind _returnvalue (Utilities|GetDataTableRow "/Game/ProjetNoel/Blueprint/Value/DT_NBG_Value.DT_NBG_Value" "FlyEnnemiHP")
    (:then
      (Variables|Default|SetHP (.value _returnvalue))
      (bind _returnvalue_2 (Utilities|GetDataTableRow "/Game/ProjetNoel/Blueprint/Value/DT_NBG_Value.DT_NBG_Value" "FlyEnnemiDamage")
        (:then
          (Variables|Default|SetDammage (.value _returnvalue_2))
          (Variables|Default|SetStartRotation (Transformation|GetActorRotation))
          (Variables|Default|SetStartLocation (Transformation|GetActorLocation))
          (Variables|/Script/Engine.InterpToMovementComponent|SetControlPoints _interptomovement (Utilities|Array|MakeArray (Utilities|Struct|MakeInterpControlPoint (Utilities|Array|Get(acopy) _locations) true) (Utilities|Struct|MakeInterpControlPoint (Utilities|Array|Get(acopy) _locations 1) true)))
          (Variables|/Script/Engine.InterpToMovementComponent|SetDuration _interptomovement 2.0))))))