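; BP_AiBase_Boss is the boss enemy, which runs the BT_BossAi behavior tree on BeginPlay.
; Its PawnSensing component sets the IsSeePlayer blackboard key to true on seeing a pawn, with no logic here to clear it.
; An OndeChoc shockwave event briefly enables overlap events on OndeCollision for half a second, and that collision stuns any NBG_HeroCharacter that begins overlapping it.
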(event OnSeePawn(PawnSensing)
  (params (Pawn :type Pawn%20Object%20Reference))
  ;[1 1 1] ifSeePlayer
  (AI|Components|Blackboard|SetValueasBool (AI|GetBlackboard (AI|GetAIController self)) (Utilities|Name|MakeLiteralName "IsSeePlayer") true))

(event OnComponentBeginOverlap(Ondecollision)
  (params (OverlappedComponent :type Primitive%20Component%20Object%20Reference) (OtherActor :type Actor%20Object%20Reference) (OtherComp :type Primitive%20Component%20Object%20Reference) (OtherBodyIndex :type Integer) (bFromSweep :type Boolean) (SweepResult :type Hit%20Result%20Structure%20%28by%20ref%29))
  (bind _asnbg_hero_character (Utilities|Casting|CastToNBG_HeroCharacter OtherActor))
  (Class|NBGHeroCharacter|Stun _asnbg_hero_character))

(event Custom|OndeChoc
  (bind _onde_collision (Variables|Default|GetOnde%20collision))
  (Variables|/Script/Engine.PrimitiveComponent|SetbGenerateOverlapEvents _onde_collision true)
  (Utilities|FlowControl|Delay 0.5)
  (Variables|/Script/Engine.PrimitiveComponent|SetbGenerateOverlapEvents _onde_collision false))

(event EventBeginPlay
  (|CallParentFunction)
  (AI|RunBehaviorTree (AI|GetAIController self) "/Game/ProjetNoel/Blueprint/Ennemi/BehaviorTree/BossAi/BT_BossAi.BT_BossAi"))

(event Collision|EventActorBeginOverlap
  (params (OtherActor :type Actor%20Object%20Reference))
  (|CallParentFunction OtherActor))

(fn ConstructionScript
  (|CallParentFunction))