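; Flying enemy pawn that runs the BT_FlyingAi behavior tree on BeginPlay.
; Its construction script loads HP and damage from DT_ValueInGame, then stores its starting rotation if both rows are found.
; PawnSensing sightings set the IsSeePlayer blackboard key, with no check on which pawn was seen, and a two-second Delay clears it.
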(event OnSeePawn(PawnSensing)
  (params (Pawn :type Pawn%20Object%20Reference))
  (bind _returnvalue (Utilities|Name|MakeLiteralName "IsSeePlayer"))
  (bind _self self)
  (bind _returnvalue_2 (AI|GetAIController _self))
  (bind _returnvalue_3 (AI|GetBlackboard _returnvalue_2))
  ;[1 1 1] ifSeePlayer
  (AI|Components|Blackboard|SetValueasBool _returnvalue_3 _returnvalue true)
  (Utilities|FlowControl|Delay 2.0)
  (AI|Components|Blackboard|SetValueasBool _returnvalue_3 _returnvalue false))

(event EventBeginPlay
  (|CallParentFunction)
  (AI|RunBehaviorTree (AI|GetAIController self) "/Game/ProjetNoel/Blueprint/Ennemi/BehaviorTree/FlyAi/BT_FlyingAi.BT_FlyingAi"))

(fn ConstructionScript
  (|CallParentFunction)
  (bind _returnvalue (Utilities|GetDataTableRow "/Game/ProjetNoel/Blueprint/Value/DT_ValueInGame.DT_ValueInGame" "FlyEnnemiHP")
    (:then
      (Variables|Default|SetHP (.value _returnvalue))
      (bind _returnvalue_2 (Utilities|GetDataTableRow "/Game/ProjetNoel/Blueprint/Value/DT_ValueInGame.DT_ValueInGame" "FlyEnnemiDmg")
        (:then
          (Variables|Default|SetDammage (.value _returnvalue_2))
          (Variables|Default|SetStartRotation (Transformation|GetActorRotation)))))))