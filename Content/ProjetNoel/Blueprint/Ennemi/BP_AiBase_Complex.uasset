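; BP_AiBase_Complex is the complex enemy AI variant, driven by the BT_ComplexAi behavior tree that its AI controller runs on BeginPlay.
; Its construction script calls the parent's, then loads HP, shoot speed and distance from the DT_NBG_Value data table through chained row lookups.
; When PawnSensing sees a pawn, it changes the State enum and sets the IsSeePlayer blackboard key to true, with nothing here clearing it.
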(event OnSeePawn(PawnSensing)
  (params (Pawn :type Pawn%20Object%20Reference))
  ;[1 1 1] ifSeePlayer
  (Variables|Default|SetState "NewEnumerator1")
  (AI|Components|Blackboard|SetValueasBool (AI|GetBlackboard (AI|GetAIController self)) (Utilities|Name|MakeLiteralName "IsSeePlayer") true))

(event EventBeginPlay
  (|CallParentFunction)
  (AI|RunBehaviorTree (AI|GetAIController self) "/Game/ProjetNoel/Blueprint/Ennemi/BehaviorTree/ComplexAI/BT_ComplexAi.BT_ComplexAi"))

(fn ConstructionScript
  (|CallParentFunction)
  (bind _returnvalue (Utilities|GetDataTableRow "/Game/ProjetNoel/Blueprint/Value/DT_NBG_Value.DT_NBG_Value" "ComplexEnnemiHP")
    (:then
      (Variables|Default|SetHP (.value _returnvalue))
      (bind _returnvalue_2 (Utilities|GetDataTableRow "/Game/ProjetNoel/Blueprint/Value/DT_NBG_Value.DT_NBG_Value" "ComplexEnnemiShootSpeed")
        (:then
          (Variables|Default|SetShootSpeed (.value _returnvalue_2))
          (bind _returnvalue_3 (Utilities|GetDataTableRow "/Game/ProjetNoel/Blueprint/Value/DT_NBG_Value.DT_NBG_Value" "ComplexEnnemiDistance")
            (:then
              (Variables|Default|SetDistance (.value _returnvalue_3)))))))))