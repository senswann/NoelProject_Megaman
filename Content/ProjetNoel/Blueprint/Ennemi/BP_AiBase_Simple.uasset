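; Simple enemy AI Blueprint that opens on seeing a pawn and fires three projectiles from arrow components.
; A state machine drives it: sight sets Opening, idle randomly picks Shoot or Closing after a delay, and OnStateChangee dispatches phase events.
; Collision is enabled only from the shoot phase until the safe phase, which re-arms sight triggering after a random delay.
; Construction reads HP from the DT_ValueInGame data table.
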(event OnSeePawn(PawnSensing)
  (params (Pawn :type Pawn%20Object%20Reference))
  ;[1 1 1] See the player
  (if (and (Utilities|Enum|NotEqual(Enum) (Variables|Default|GetState) "NewEnumerator1") (Variables|Default|GetIfNotShoot))
    (Variables|Default|SetState "NewEnumerator3")))

(event Custom|ShootEvent
  ;[1 1 1] Shoot phase
  (Variables|Default|SetIfNotShoot false)
  (Collision|SetCollisionEnabled (Variables|Default|GetCollision) "QueryAndPhysics")
  (CallFunction|Shoot (Variables|Default|GetShootArrow))
  (CallFunction|Shoot (Variables|Default|GetShootArrow1))
  (CallFunction|Shoot (Variables|Default|GetShootArrow2)))

(event Custom|SafeEvent
  ;[1 1 1] Safe phase
  (Collision|SetCollisionEnabled (Variables|Default|GetCollision) "NoCollision")
  (Utilities|FlowControl|Delay (Math|Random|RandomFloatinRange 0.5 3.0))
  (Variables|Default|SetIfNotShoot true))

(event Custom|IdleShoot
  (Utilities|FlowControl|Delay (Math|Random|RandomFloatinRange 0.5 3.0))
  (if (Math|Random|RandomBool)
    (Variables|Default|SetState "NewEnumerator1")
    (else
      (Variables|Default|SetState "NewEnumerator2")))
  (CallFunction|OnStateChangee))

(event EventBeginPlay
  (|CallParentFunction)
  (CallFunction|SafeEvent))

(event Collision|EventActorBeginOverlap
  (params (OtherActor :type Actor%20Object%20Reference))
  (|CallParentFunction OtherActor) ; This node is disabled and will not be called.\nDrag off pins to build functionality.
)

(event EventTick
  (params (DeltaSeconds :type Float%20%28single-precision%29))
  (|CallParentFunction DeltaSeconds) ; This node is disabled and will not be called.\nDrag off pins to build functionality.
)

(fn ConstructionScript
  (|CallParentFunction)
  (bind _returnvalue (Utilities|GetDataTableRow "/Game/ProjetNoel/Blueprint/Value/DT_ValueInGame.DT_ValueInGame" "SimpleEnnemiHP")
    (:then
      (Variables|Default|SetHP (.value _returnvalue)))))

(fn Shoot
  (params (SpawnShoot :type Arrow%20Component%20Object%20Reference))
  (Game|SpawnActorfromClass "/Game/ProjetNoel/Blueprint/Items/BP_Projectile.BP_Projectile_C" (Math|Transform|MakeTransform (Transformation|GetWorldLocation SpawnShoot) (Transformation|GetWorldRotation SpawnShoot) "1.000000,1.000000,1.000000") "Undefined" "MultiplyWithRoot" self 0))

(fn OnStateChangee
  (switch Utilities|FlowControl|Switch|SwitchonE_AISimple (Variables|Default|GetState)
    (:NewEnumerator0
      (CallFunction|SafeEvent))
    (:NewEnumerator1
      (CallFunction|ShootEvent))
    (:NewEnumerator4
      (CallFunction|IdleShoot))))