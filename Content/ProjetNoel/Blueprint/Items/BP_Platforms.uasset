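; BP_Platforms is a moving platform actor driven by an InterpToMovement component.
; The construction script builds two relative control points from the Location array and applies the Duration variable, so path and timing come from variables.
; OpenPlatform toggles OpenPlatformBool and swaps the static mesh material between green and an alternate, without touching the movement.
; The event graph holds no active logic.
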(event EventBeginPlay)

(event Collision|EventActorBeginOverlap
  (params (OtherActor :type Actor%20Object%20Reference)))

(event EventTick
  (params (DeltaSeconds :type Float%20%28single-precision%29)))

(fn ConstructionScript
  (bind _interptomovement (Variables|Default|GetInterpToMovement))
  (bind _location (Variables|Default|GetLocation))
  (Variables|/Script/Engine.InterpToMovementComponent|SetControlPoints _interptomovement (Utilities|Array|MakeArray (Utilities|Struct|MakeInterpControlPoint (Utilities|Array|Get(acopy) _location) true) (Utilities|Struct|MakeInterpControlPoint (Utilities|Array|Get(acopy) _location 1) true)))
  (Variables|/Script/Engine.InterpToMovementComponent|SetDuration _interptomovement (Variables|Default|GetDuration)))

(fn OpenPlatform
  (bind _staticmesh (Variables|Default|GetStaticMesh))
  (if (Variables|Default|GetOpenPlatformBool)
    (Rendering|Material|SetMaterial _staticmesh 0 "/DatasmithContent/Materials/AliasReference.AliasReference")
    (Variables|Default|SetOpenPlatformBool false)
    (else
      (Rendering|Material|SetMaterial _staticmesh 0 "/AnimationSharing/AnimSharingGreen.AnimSharingGreen")
      (Variables|Default|SetOpenPlatformBool true))))