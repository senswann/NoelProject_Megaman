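; BP_HealBoost is a health bonus pickup for the hero character.
; Its construction script reads HpRecovery from DT_ValueInGame, choosing the medium or low life bonus row through the HPMedium flag.
; When a BP_HeroCharacter overlaps its static mesh, it passes that value to the hero's SetHP and destroys itself.
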(event OnComponentBeginOverlap(StaticMesh)
  (params (OverlappedComponent :type Primitive%20Component%20Object%20Reference) (OtherActor :type Actor%20Object%20Reference) (OtherComp :type Primitive%20Component%20Object%20Reference) (OtherBodyIndex :type Integer) (bFromSweep :type Boolean) (SweepResult :type Hit%20Result%20Structure%20%28by%20ref%29))
  (bind _asbp_hero_character (Utilities|Casting|CastToBP_HeroCharacter OtherActor))
  (Default|SetHP _asbp_hero_character (Variables|Default|GetHpRecovery))
  (Actor|DestroyActor))

(fn ConstructionScript
  (if (Variables|Default|GetHPMedium)
    (bind _returnvalue (Utilities|GetDataTableRow "/Game/ProjetNoel/Blueprint/Value/DT_ValueInGame.DT_ValueInGame" "MediumLifeBonus")
      (:then
        (Variables|Default|SetHpRecovery (.value _returnvalue))))
    (else
      (bind _returnvalue_2 (Utilities|GetDataTableRow "/Game/ProjetNoel/Blueprint/Value/DT_ValueInGame.DT_ValueInGame" "LowLifeBonus")
        (:then
          (Variables|Default|SetHpRecovery (.value _returnvalue_2)))))))