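; BP_Projectile is a projectile item that configures its speed and damage from the DT_ValueInGame data table.
; Its construction script applies the ShootSpeed row to both initial and max speed of the ProjectileMovement component.
; It then switches on the owner's class display name to load Damage from either the player row for the hero or the simple-enemy row for the basic AI.
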(fn ConstructionScript
  (bind _projectilemovement (Variables|Default|GetProjectileMovement))
  (bind _returnvalue (Utilities|GetDataTableRow "/Game/ProjetNoel/Blueprint/Value/DT_ValueInGame.DT_ValueInGame" "ShootSpeed")
    (:then
      (Variables|/Script/Engine.ProjectileMovementComponent|SetInitialSpeed _projectilemovement (Math|Conversions|ToFloat(Integer) (.value _returnvalue)))
      (Variables|/Script/Engine.ProjectileMovementComponent|SetMaxSpeed _projectilemovement (Math|Conversions|ToFloat(Integer) (.value _returnvalue)))
      (switch string (Utilities|GetClassDisplayName (Utilities|GetClass (Components|GetOwner)))
        (:BP_HeroCharacter_C
          (bind _returnvalue_2 (Utilities|GetDataTableRow "/Game/ProjetNoel/Blueprint/Value/DT_ValueInGame.DT_ValueInGame" "DamageJoueur")
            (:then
              (Variables|Default|SetDamage (.value _returnvalue_2)))))
        (:BP_AiBase_Simple_C
          (bind _returnvalue_3 (Utilities|GetDataTableRow "/Game/ProjetNoel/Blueprint/Value/DT_ValueInGame.DT_ValueInGame" "SimpleEnnemiDamage")
            (:then
              (Variables|Default|SetDamage (.value _returnvalue_3)))))))))